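; TV is an actor that shows a descriptive text prompt above itself when the player comes near.
; On BeginPlay it creates an InteractUI widget with its Description and a position offset, adds it to the viewport, and removes it when destroyed.
; Begin overlap sets the text visible only if the other actor is the player pawn.
; Any end overlap hides it, regardless of which actor leaves.
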(event `self.ReceiveActorEndOverlap`
  (params (OtherActor :type "Actor Object Reference"))
  ;[1 1 1] Make Invisible when player goes further away.
  (`/Game/Blueprints/InteractUI.SetTextVisibility` (`self.UI`) false))

(event `self.ReceiveActorBeginOverlap`
  (params (OtherActor :type "Actor Object Reference"))
  ;[1 1 1] Make visible when player comes near
  (`/Game/Blueprints/InteractUI.SetTextVisibility` (`self.UI`) (== OtherActor (`GameplayStatics.GetPlayerPawn` 0))))

(event `self.ReceiveBeginPlay`
  ;[1 1 1] Create Text Above Actor
  (bind _returnvalue (`|CreateWidget` "/Game/Blueprints/InteractUI.InteractUI_C" null self (`self.Description`) (10.0 0.0 50.0)))
  (set `self.UI` _returnvalue)
  (`UserWidget.AddToViewport` _returnvalue 0))

(event `self.ReceiveDestroyed`
  ;[1 1 1] Remove Text on Destroy
  (`Widget.RemoveFromParent` (`self.UI`)))

(fn `UserConstructionScript`)