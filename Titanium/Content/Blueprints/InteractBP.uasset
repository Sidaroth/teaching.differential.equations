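; InteractBP handles player interaction with dead bodies and exit doors.
; On BeginPlay it creates an on-screen text widget, and AttemptInteract line-traces from the camera along its view up to Reach.
; The hit actor's display name selects the action: a body's temperature is printed and sent to the HUD, while the door opens NextLevel.
; A timer calls OnFade to hide the HUD text three seconds after a body check.
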(event `self.ReceiveBeginPlay`
  (bind _returnvalue (`|CreateWidget` "/Game/Blueprints/OnScreenText_BP.OnScreenText_BP_C"))
  (bind _output_get (set `self.HUDRef` _returnvalue))
  (`UserWidget.AddToViewport` _output_get 0))

(event `OnFade`
  (set `/Game/Blueprints/OnScreenText_BP.TextVisibility` false (`self.HUDRef`)))

(fn `AttemptInteract`
  (bind _transformcomponent (`PlayerCameraManager.TransformComponent` (`GameplayStatics.GetPlayerCameraManager` 0)))
  (bind _returnvalue (`SceneComponent.K2_GetComponentLocation` _transformcomponent))
  (bind _outhit (`KismetSystemLibrary.LineTraceSingle` :`Start` _returnvalue :`End` (+ _returnvalue (* (`KismetMathLibrary.GetForwardVector` (`SceneComponent.K2_GetComponentRotation` _transformcomponent)) (`self.Reach`))) :`TraceChannel` "TraceTypeQuery1" :`DrawDebugType` "ForOneFrame"))
  (bind (_bblockinghit _binitialoverlap _time _location _impactpoint _normal _impactnormal _physmat _hitactor) (`GameplayStatics.BreakHitResult` _outhit))
  ;[1 1 1] See what we hit and act accordingly
  (switch `string` (`KismetSystemLibrary.GetDisplayName` _hitactor)
    (:`DeadBody1`
      (`self.InteractWithBody` _hitactor))
    (:`ExitDoor1`
      (`self.InteractWithDoor`))))

(fn `InteractWithBody`
  (params (Body :type "Actor Object Reference"))
  (bind _returnvalue (`KismetStringLibrary.Conv_DoubleToString` (`Temperature.BodyTemperature` (`Actor.GetComponentByClass` Body "/Script/Titanium.Temperature"))))
  (`KismetSystemLibrary.PrintString` _returnvalue false)
  (`/Game/Blueprints/OnScreenText_BP.UpdateContent` (`self.HUDRef`) (`KismetSystemLibrary.MakeLiteralString` _returnvalue))
  ;[1 1 1] Make invisible after 3 seconds
  (`KismetSystemLibrary.K2_SetTimer` self "OnFade" 3.0))

(fn `InteractWithDoor`
  (`GameplayStatics.OpenLevel` (`self.NextLevel`)))