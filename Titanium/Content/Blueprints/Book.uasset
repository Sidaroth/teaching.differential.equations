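; Book is an interactable clue prop that shows a flavor line about the victim's reading habits when the player is near.
; On BeginPlay it creates an InteractUI widget with that text and a small vertical offset, then adds it to the viewport.
; Overlap begin shows the text only for the player pawn, any overlap end hides it, and destruction removes the widget.
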(event `self.ReceiveActorEndOverlap`
  (params (OtherActor :type "Actor Object Reference"))
  ;[1 1 1] Make Invisible when player goes further away.
  (`/Game/Blueprints/InteractUI.SetTextVisibility` (`self.UIText`) false))

(event `self.ReceiveActorBeginOverlap`
  (params (OtherActor :type "Actor Object Reference"))
  ;[1 1 1] Make visible when player comes near
  (`/Game/Blueprints/InteractUI.SetTextVisibility` (`self.UIText`) (== OtherActor (`GameplayStatics.GetPlayerPawn` 0))))

(event `self.ReceiveBeginPlay`
  ;[1 1 1] Create the widget with the appropriate text, make a reference for later use.
  (bind _returnvalue (`|CreateWidget` "/Game/Blueprints/InteractUI.InteractUI_C" null self "The victim seems to be an avid reader. " (0.0 0.0 10.0)))
  (bind _output_get (set `self.UIText` _returnvalue))
  (`UserWidget.AddToViewport` _output_get 0))

(event `self.ReceiveDestroyed`
  ;[1 1 1] Remove reference on delete
  (`Widget.RemoveFromParent` (`self.UIText`)))

(fn `UserConstructionScript`)